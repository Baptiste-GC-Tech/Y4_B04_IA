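; Enemy AI controller that detects the player through AI Perception and drives an enemy behavior tree.
; On play it sets up the blackboard and runs BT_EnnemyBehavior.
; Perception updates write player-in-sight and an AI state enum to the blackboard, switching state when sensed and reverting via a stimulus-age timer or when forgotten, then notifying of the change.
; Debug prints show detection events and the current suspicion level each tick.
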(event OnTargetPerceptionUpdated(AIPerception)
  (params (Actor :type Actor%20Object%20Reference) (Stimulus :type AI%20Stimulus%20Structure))
  (bind (_age _expirationage _strength _stimuluslocation _receiverlocation _tag _bsuccessfullysensed) (Utilities|Struct|BreakAIStimulus Stimulus))
  ;[0.15 0.15 0.15 0.5] Makes sure we've percepted the Player
  (Development|PrintString (Utilities|GetObjectName Actor))
  (Utilities|Casting|CastToBP_ThirdPersonCharacter Actor
    (:then
      (AI|Components|Blackboard|SetValueasBool (Variables|Default|GetBlackBoardComp) (Utilities|Name|MakeLiteralName "IsPlayerInSight") _bsuccessfullysensed)
      (if _bsuccessfullysensed
        (AI|Components|Blackboard|SetValueasEnum (Variables|Default|GetBlackBoardComp) (Variables|Default|GetStateEnumName) (Utilities|Enum|LiteralenumEAIState "NewEnumerator1"))
        (Default|CallOnEnumStateChange)
        (Development|PrintString "Player detected" true true "(R=0.000000,G=1.000000,B=0.000000,A=1.000000)")
        (else
          (Utilities|Time|SetTimerbyEvent (delegate Custom|CallBack) _expirationage))))
    (:CastFailed
      (Development|PrintString "No player detected" true true "(R=1.000000,G=0.000000,B=0.000000,A=1.000000)" 4.0))))

(event OnTargetPerceptionForgotten(AIPerception)
  (params (Actor :type Actor%20Object%20Reference))
  (Utilities|Casting|CastToBP_ThirdPersonCharacter Actor)
  (AI|Components|Blackboard|SetValueasEnum (Variables|Default|GetBlackBoardComp) (Variables|Default|GetStateEnumName) (Utilities|Enum|LiteralenumEAIState "NewEnumerator0"))
  (Default|CallOnEnumStateChange))

(event Custom|CallBack
  (bind _blackboardcomp (Variables|Default|GetBlackBoardComp))
  (bind _stateenumname (Variables|Default|GetStateEnumName))
  (if (.bSuccessfullySensed (Utilities|Struct|BreakAIStimulus (stale OnTargetPerceptionUpdated(AIPerception) Stimulus)))
    (AI|Components|Blackboard|SetValueasEnum _blackboardcomp _stateenumname (Utilities|Enum|LiteralenumEAIState "NewEnumerator1"))
    (Default|CallOnEnumStateChange)
    (Development|PrintString "Player detected" true true "(R=0.000000,G=1.000000,B=0.000000,A=1.000000)")
    (else
      (AI|Components|Blackboard|SetValueasEnum _blackboardcomp _stateenumname (Utilities|Enum|LiteralenumEAIState "NewEnumerator0"))
      (Default|CallOnEnumStateChange)
      (Development|PrintString "Player Unseen" true true "(R=0.000000,G=1.000000,B=0.000000,A=1.000000)"))))

(event Custom|CustomEvent)

(event EventBeginPlay
  (bind _blackboardcomponent (Class|AIController|UseBlackboard (Variables|Default|GetBlackBoardData)))
  (Variables|Default|SetBlackBoardComp _blackboardcomponent)
  (AI|RunBehaviorTree "/Game/Leo/Behaviors/BT_EnnemyBehavior.BT_EnnemyBehavior"))

(event EventTick
  (params (DeltaSeconds :type Float%20%28single-precision%29))
  (Development|PrintString (Utilities|String|Append "Detection level : " (Utilities|String|ToString(Float) (Class|BlackboardComponent|GetValueasFloat (Variables|Default|GetBlackBoardComp) (Utilities|Name|MakeLiteralName "SuspicionLevel")))) true true "(R=0.000000,G=0.660000,B=1.000000,A=1.000000)" DeltaSeconds))

(fn ConstructionScript)