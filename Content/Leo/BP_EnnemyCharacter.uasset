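; Enemy character whose spotlight color signals its AI state: patrol, alert or combat.
; The construction script assigns BP_EnnemyAIController as its AI controller class.
; On possession it binds to the controller's enum state change event, then reads the blackboard State key and recolors the spotlight to match.
; Debug strings report possession, color changes and wrong-controller casts.
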(event Custom|StateEnumCallback
  (bind _spotlight (Variables|Default|GetSpotLight))
  (bind _asbp_ennemy_aicontroller (Utilities|Casting|CastToBP_EnnemyAIController (Pawn|GetController))
    (:then
      ;[0.15 0.15 0.15 0.5] Switch the light color
      (switch Utilities|FlowControl|Switch|SwitchonEAIState (Utilities|Enum|ByteToEnumEAIState (Class|BlackboardComponent|GetValueasEnum (AI|GetBlackboard _asbp_ennemy_aicontroller) (Utilities|Name|MakeLiteralName "State")))
        (:NewEnumerator0
          (Rendering|Components|Light|SetLightColor _spotlight (Variables|Default|GetBaseColor) true)
          (Development|PrintString "Light color set to White"))
        (:NewEnumerator1
          (Rendering|Components|Light|SetLightColor _spotlight (Variables|Default|GetAlertColor) true)
          (Development|PrintString "Light color set to Yellow"))
        (:NewEnumerator2
          (Rendering|Components|Light|SetLightColor _spotlight (Variables|Default|GetCombatColor) true)
          (Development|PrintString "Light color set to Red"))))
    (:CastFailed
      (Development|PrintString "Not the good AI controller" true true "(R=1.000000,G=0.000000,B=0.000000,A=1.000000)" 4.0))))

(event EventPossessed
  (params (NewController :type Controller%20Object%20Reference))
  (Development|PrintString (Utilities|String|Append "Possessed by : " (Utilities|GetObjectName NewController)) true true "(R=0.207569,G=1.000000,B=0.405902,A=1.000000)" 4.0)
  (bind _asbp_ennemy_aicontroller (Utilities|Casting|CastToBP_EnnemyAIController (Pawn|GetController))
    (:then
      (EventDispatchers|BindEventtoOnEnumStateChange _asbp_ennemy_aicontroller (delegate Custom|StateEnumCallback)))
    (:CastFailed
      (Development|PrintString "Not the good AI Controller" true true "(R=1.000000,G=0.000000,B=0.000000,A=1.000000)" 4.0))))

(fn ConstructionScript
  (Variables|Default|SetAIControllerClass "/Game/Leo/Behaviors/BP_EnnemyAIController.BP_EnnemyAIController_C"))