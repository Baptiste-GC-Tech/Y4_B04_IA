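; Enemy AI controller that starts the enemy behavior tree on BeginPlay.
; It initializes the blackboard and writes a one-time target vector a short distance in front of the player pawn before running BT_EnnemyBehavior.
; A looping retarget timer and a missing-key debug print are left unconnected, and SetNewTarget is empty, so the controller never refreshes the target.
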(event Custom|SetNewTarget)

(event EventBeginPlay
  (bind _returnvalue (Game|Player|GetPlayerPawn 0))
  (bind _blackboardcomponent (Class|AIController|UseBlackboard (Variables|Default|GetBlackBoardComp)))
  (AI|Components|Blackboard|SetValueasVector _blackboardcomponent (Variables|Default|GetTargetKeyName) (+ (Transformation|GetActorLocation _returnvalue) (* (Transformation|GetActorForwardVector _returnvalue) (Math|Float|MakeLiteralFloat 8e+01))))
  (AI|RunBehaviorTree "/Game/Leo/BT_EnnemyBehavior.BT_EnnemyBehavior"))

(fn ConstructionScript)