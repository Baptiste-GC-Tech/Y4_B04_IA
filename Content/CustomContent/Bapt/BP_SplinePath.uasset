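; BP_SplinePath is a spline actor that moves an indicator component, PosByTimeIndicator, along its spline in a loop.
; Each Tick adds delta time to an elapsed timer, multiplies it by IndicatorSpeedUnits to get a distance, and places the indicator at that local spline location.
; The timer resets to zero once that distance reaches the spline length.
; It also prints timing debug text every frame and contains unused experimental index-stepping logic.
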(event EventBeginPlay)

(event EventTick
  (params (DeltaSeconds :type Float%20%28single-precision%29))
  (Development|PrintString (Utilities|String|Append "Delta: " (Utilities|String|ToString(Float) DeltaSeconds) "  |  SinceStart: " (Utilities|String|ToString(Float) (Variables|Default|GetTimeAlongSpline))))
  ;[0.15 0.15 0.15 0.5] Update time elapsed and proceed if this didn't go over spline's duration. If above, resets it (loop)
  (Variables|Default|SetTimeAlongSpline (+ (Variables|Default|GetTimeAlongSpline) DeltaSeconds))
  (if (>= (* (Variables|Default|GetTimeAlongSpline) (Variables|Default|GetIndicatorSpeed%20%28unit/s%29)) (Spline|GetSplineLength (Variables|Default|GetSpline)))
    (Variables|Default|SetTimeAlongSpline 0.0))
  (Transformation|SetRelativeLocation (Variables|Default|GetPosByTimeIndicator) (Spline|GetLocationatDistanceAlongSpline (Variables|Default|GetSpline) (* (Variables|Default|GetTimeAlongSpline) (Variables|Default|GetIndicatorSpeed%20%28unit/s%29)) "Local") false false))

(fn ConstructionScript)