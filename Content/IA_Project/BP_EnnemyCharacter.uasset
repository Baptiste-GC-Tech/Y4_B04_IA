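; Enemy AI character that shows its awareness state through a spotlight, a sight-sense widget and its movement speed.
; On possession by BP_EnnemyAIController, it binds to the controller's state-change event and reads the State enum from the blackboard.
; Patrol, Alert and Combat set light color and walk speed, while the widget color changes only for Alert and Combat.
; Each tick, it copies the blackboard SuspicionLevel into the widget.
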(event Custom|StateEnumCallback
  (bind __controller (Variables|Default|Get_controller))
  (bind _returnvalue (CallFunction|GetStateEnum __controller))
  ;[0.15 0.15 0.15 0.5] Enum callback functions
  (CallFunction|HandleLightColor _returnvalue)
  (CallFunction|HandleWidgetColor _returnvalue)
  (CallFunction|HandleCharacterSpeed _returnvalue (Variables|AI|GetWalkSpeed) (Variables|AI|GetFastWalkSpeed) (Variables|AI|GetRunSpeed)))

(event EventTick
  (params (DeltaSeconds :type Float%20%28single-precision%29))
  ;[0.004968 0.08617 0.15 0.5] Update the widget value
  (bind _aswbp_sight_sense_value (Utilities|Casting|CastToWBP_SightSenseValue (UserInterface|GetWidget (Variables|Default|GetSightWidget))))
  (Variables|/Game/IA_Project/WBP_SightSenseValue.WBP_SightSenseValue_C|SetSightValue _aswbp_sight_sense_value (Class|BlackboardComponent|GetValueasFloat (AI|GetBlackboard (Variables|Default|Get_controller)) (Utilities|Name|MakeLiteralName "SuspicionLevel"))))

(event EventBeginPlay
  (Variables|/Script/Engine.CharacterMovementComponent|SetMaxWalkSpeed (Variables|Character|GetCharacterMovement) (Variables|AI|GetWalkSpeed)))

(event EventPossessed
  (params (NewController :type Controller%20Object%20Reference))
  (Development|PrintString (Utilities|String|Append "Possessed by : " (Utilities|GetObjectName NewController)) true true "(R=0.207569,G=1.000000,B=0.405902,A=1.000000)" 4.0)
  (bind _asbp_ennemy_aicontroller (Utilities|Casting|CastToBP_EnnemyAIController (Pawn|GetController))
    (:then
      (bind _output_get (Variables|Default|Set_controller _asbp_ennemy_aicontroller))
      (EventDispatchers|BindEventtoOnEnumStateChange _output_get (delegate Custom|StateEnumCallback)))
    (:CastFailed
      (Development|PrintString "Not the good AI Controller" true true "(R=1.000000,G=0.000000,B=0.000000,A=1.000000)" 4.0))))

(fn ConstructionScript
  (Variables|Default|SetAIControllerClass "/Game/IA_Project/Behaviors/BP_EnnemyAIController.BP_EnnemyAIController_C"))

(fn GetStateEnum
  (params (Target :type Actor%20Object%20Reference))
  (return (Utilities|Enum|ByteToEnumEAIState (Class|BlackboardComponent|GetValueasEnum (AI|GetBlackboard Target) (Utilities|Name|MakeLiteralName "State")))))

(fn HandleLightColor
  (params (newState :type EAIState%20Enum :default "NewEnumerator0"))
  (bind _spotlight (Variables|Default|GetSpotLight))
  (switch Utilities|FlowControl|Switch|SwitchonEAIState newState
    (:NewEnumerator0
      (Rendering|Components|Light|SetLightColor _spotlight (Variables|AI|GetBaseColor) true))
    (:NewEnumerator1
      (Rendering|Components|Light|SetLightColor _spotlight (Variables|AI|GetAlertColor) true))
    (:NewEnumerator2
      (Rendering|Components|Light|SetLightColor _spotlight (Variables|AI|GetCombatColor) true))))

(fn HandleWidgetColor
  (params (newState :type EAIState%20Enum :default "NewEnumerator0"))
  (bind _aswbp_sight_sense_value (Utilities|Casting|CastToWBP_SightSenseValue (UserInterface|GetWidget (Variables|Default|GetSightWidget))))
  (switch Utilities|FlowControl|Switch|SwitchonEAIState newState
    (:NewEnumerator1
      (Variables|/Game/IA_Project/WBP_SightSenseValue.WBP_SightSenseValue_C|SetColor _aswbp_sight_sense_value (Variables|AI|GetAlertColor)))
    (:NewEnumerator2
      (Variables|/Game/IA_Project/WBP_SightSenseValue.WBP_SightSenseValue_C|SetColor _aswbp_sight_sense_value (Variables|AI|GetCombatColor)))))

(fn HandleCharacterSpeed
  (params (newState :type EAIState%20Enum :default "NewEnumerator0") (WalkSpeed :type Float%20%28double-precision%29) (FastWalkSpeed :type Float%20%28double-precision%29) (RunSpeed :type Float%20%28double-precision%29))
  (bind _charactermovement (Variables|Character|GetCharacterMovement))
  (switch Utilities|FlowControl|Switch|SwitchonEAIState newState
    (:NewEnumerator0
      (Variables|/Script/Engine.CharacterMovementComponent|SetMaxWalkSpeed _charactermovement WalkSpeed))
    (:NewEnumerator1
      (Variables|/Script/Engine.CharacterMovementComponent|SetMaxWalkSpeed _charactermovement FastWalkSpeed))
    (:NewEnumerator2
      (Variables|/Script/Engine.CharacterMovementComponent|SetMaxWalkSpeed _charactermovement RunSpeed))))