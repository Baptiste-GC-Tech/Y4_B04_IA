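; Enemy AI controller that runs the BT_EnnemyBehavior tree and feeds it player perception through the blackboard.
; Perception updates set IsPlayerInSight (player only) and IsPlayerHeard, and write every stimulus location to TargetLocation.
; Tick prints debug values for suspicion and both senses, and refreshes TargetLocation via GetLastPlayerLocation while sighted, though that function's lookup is unconnected.
; SetStateEnum writes the blackboard state and signals the change.
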(event OnTargetPerceptionUpdated(AIPerception)
  (params (Actor :type Actor%20Object%20Reference) (Stimulus :type AI%20Stimulus%20Structure))
  ;[0.15 0.15 0.15 0.5] Makes sure we've percepted the Player
  (Development|PrintString (Utilities|GetObjectName Actor))
  (CallFunction|HandleAIPerception Actor Stimulus))

(event EventBeginPlay
  ;[0.15 0.15 0.15 0.5] Initialisation
  (bind _blackboardcomponent (Class|AIController|UseBlackboard (Variables|AI|GetBlackBoardData)))
  (Variables|AI|SetBlackBoardComp _blackboardcomponent)
  (AI|RunBehaviorTree "/Game/IA_Project/Behaviors/BT_EnnemyBehavior.BT_EnnemyBehavior"))

(event EventTick
  (params (DeltaSeconds :type Float%20%28single-precision%29))
  ;[0.15 0.15 0.15 0.5] Tick update
  (CallFunction|DebugSightLevel DeltaSeconds)
  (CallFunction|DebugIsPlayerinSight DeltaSeconds)
  (CallFunction|DebugIsPlayerHeard DeltaSeconds)
  (if (ScalableFloat|GetValueasBool (Variables|AI|GetBlackBoardComp) (Utilities|Name|MakeLiteralName "IsPlayerInSight"))
    (AI|Components|Blackboard|SetValueasVector (Variables|AI|GetBlackBoardComp) (Utilities|Name|MakeLiteralName "TargetLocation") (Utilities|GetLastPlayerLocation))))

(fn ConstructionScript)

(fn SetStateEnum
  (params (newState :type EAIState%20Enum :default "NewEnumerator0"))
  (AI|Components|Blackboard|SetValueasEnum (Variables|AI|GetBlackBoardComp) (Variables|AI|GetStateEnumName) newState)
  (Default|CallOnEnumStateChange))

(fn DebugSightLevel
  (params (Duration :type Float%20%28single-precision%29))
  (Development|PrintString (Utilities|String|Append "Detection level : " (Utilities|String|ToString(Float) (Class|BlackboardComponent|GetValueasFloat (Variables|AI|GetBlackBoardComp) (Utilities|Name|MakeLiteralName "SuspicionLevel")))) true false "(R=0.000000,G=0.660000,B=1.000000,A=1.000000)" Duration))

(fn HandleAIPerception
  (params (StimulusActorSource :type Actor%20Object%20Reference) (AIStimulus :type AI%20Stimulus%20Structure%20%28by%20ref%29))
  (bind (_age _expirationage _strength _stimuluslocation _receiverlocation _tag _bsuccessfullysensed) (Utilities|Struct|BreakAIStimulus AIStimulus))
  (bind _blackboardcomp (Variables|AI|GetBlackBoardComp))
  (Utilities|FlowControl|Sequence
    (:then_0
      ;[0.15 0.15 0.15 0.5] Saves in BB if Sight Sense triggered
      (Utilities|Casting|CastToBP_ThirdPersonCharacter StimulusActorSource)
      (bind _returnvalue (Class|AIPerceptionSystem|GetSenseClassforStimulus AIStimulus))
      (AI|Components|Blackboard|SetValueasBool (Variables|AI|GetBlackBoardComp) (Utilities|Name|MakeLiteralName "IsPlayerInSight") (and (== _returnvalue "/Script/AIModule.AISense_Sight") _bsuccessfullysensed))
      (if (and (== _returnvalue "/Script/AIModule.AISense_Sight") _bsuccessfullysensed)
        (Development|PrintString "Controller detected the sense of SIGHT" true false "(R=0.463894,G=1.000000,B=0.138448,A=1.000000)" 7.0)))
    (:then_1
      ;[0.15 0.15 0.15 0.5] Saves in BB if Hearing Sense triggered
      (bind _returnvalue_2 (Class|AIPerceptionSystem|GetSenseClassforStimulus AIStimulus))
      (AI|Components|Blackboard|SetValueasBool _blackboardcomp (Utilities|Name|MakeLiteralName "IsPlayerHeard") (and (== _returnvalue_2 "/Script/AIModule.AISense_Hearing") _bsuccessfullysensed)) ; Update IsPlayerHeard
      (AI|Components|Blackboard|SetValueasVector _blackboardcomp (Utilities|Name|MakeLiteralName "TargetLocation") _stimuluslocation) ; Set the noise's location as TargetLocation
      (if (and (== _returnvalue_2 "/Script/AIModule.AISense_Hearing") _bsuccessfullysensed)
        (Development|PrintString (Utilities|String|Append "Controller detected the sense of HEARING w/ instigator " (Utilities|GetDisplayName StimulusActorSource)) true false "(R=0.554312,G=1.000000,B=0.290609,A=1.000000)" 7.0)))))

(fn DebugIsPlayerinSight
  (params (Duration :type Float%20%28single-precision%29))
  (Development|PrintString (Utilities|String|Append "BB IsPlayerInSight : " (Utilities|String|ToString(Boolean) (ScalableFloat|GetValueasBool (Variables|AI|GetBlackBoardComp) (Utilities|Name|MakeLiteralName "IsPlayerInSight")))) true false "(R=0.000000,G=0.660000,B=1.000000,A=1.000000)" Duration))

(fn DebugIsPlayerHeard
  (params (Duration :type Float%20%28single-precision%29))
  (Development|PrintString (Utilities|String|Append "BB IsPlayerHeard : " (Utilities|String|ToString(Boolean) (ScalableFloat|GetValueasBool (Variables|AI|GetBlackBoardComp) (Utilities|Name|MakeLiteralName "IsPlayerHeard")))) true false "(R=0.000000,G=0.660000,B=1.000000,A=1.000000)" Duration))